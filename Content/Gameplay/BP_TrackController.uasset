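; Track controller that runs an endless scrolling track of BP_TrackSegment actors with asteroid obstacles.
; BeginPlay lays out segments along X, keeping the first stretch obstacle-free, and Tick passes TrackSpeed to each segment's UpdateLocation.
; Segments leaving TrackRemoveTrigger are destroyed and replaced beyond the last one, with obstacles.
; TrackSpeed eases toward TopSpeed through a small Lerp run once per segment each tick, making acceleration frame-rate dependent.
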(event OnComponentEndOverlap(TrackRemoveTrigger)
  (params (OverlappedComponent :type Primitive%20Component%20Object%20Reference) (OtherActor :type Actor%20Object%20Reference) (OtherComp :type Primitive%20Component%20Object%20Reference) (OtherBodyIndex :type Integer))
  (bind _tracksegments (Variables|Default|GetTrackSegments))
  (bind _asbp_track_segment (Utilities|Casting|CastToBP_TrackSegment OtherActor))
  (Utilities|Array|RemoveItem (Variables|Default|GetTrackSegments) _asbp_track_segment)
  (Actor|DestroyActor OtherActor)
  (CallFunction|AddTrackSegment (+ (.X (Math|Vector|BreakVector (Transformation|GetWorldLocation (Variables|/Game/Gameplay/BP_TrackSegment.BP_TrackSegment_C|GetDefaultSceneRoot (Utilities|Array|Get(acopy) _tracksegments (Utilities|Array|LastIndex _tracksegments)))))) 1e+03) true))

(event EventBeginPlay
  (for _index (range -1 50)
    (CallFunction|AddTrackSegment (* _index 1e+03) (> _index 5))))

(event Collision|EventActorBeginOverlap
  (params (OtherActor :type Actor%20Object%20Reference)))

(event EventTick
  (params (DeltaSeconds :type Float%20%28single-precision%29))
  (for _array_element (Variables|Default|GetTrackSegments)
    (Default|UpdateLocation _array_element (Math|Vector|MakeVector (Variables|Default|GetTrackSpeed) 0.0 0.0))
    (CallFunction|IncrementSpeed)))

(fn ConstructionScript)

(fn AddTrackSegment
  (params (StartDistance :type Float%20%28single-precision%29) (SpawnAsteroids :type Boolean))
  (bind _returnvalue (Game|SpawnActorfromClass "/Game/Gameplay/BP_TrackSegment.BP_TrackSegment_C" (Math|Transform|MakeTransform (Math|Vector|MakeVector StartDistance 0.0 0.0)) "Undefined" 0 0))
  (Utilities|Array|Add (Variables|Default|GetTrackSegments) _returnvalue)
  (if SpawnAsteroids
    (Default|SpawnObstacles _returnvalue)))

(fn IncrementSpeed
  (Variables|Default|SetTrackSpeed (Math|Float|Lerp (Variables|Default|GetTrackSpeed) (Variables|Default|GetTopSpeed) 0.001)))