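; Track segment actor that populates itself with asteroid obstacles and moves together with them.
; SpawnObstacles spawns a small random number of BP_Asteroid actors at random X/Y offsets from the segment's root and stores them in an Asteroids array.
; UpdateLocation applies a delta offset, despite its Location parameter name, to the root and each stored asteroid's component, since the asteroids are not attached.
; Event graph and construction script are empty, so both functions rely on external calls.
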(event EventBeginPlay)

(event Collision|EventActorBeginOverlap
  (params (OtherActor :type Actor%20Object%20Reference)))

(event EventTick
  (params (DeltaSeconds :type Float%20%28single-precision%29)))

(fn ConstructionScript)

(fn SpawnObstacles
  (for _index (range 0 (Math|Random|RandomIntegerinRange 0 2))
    (bind _returnvalue (Game|SpawnActorfromClass "/Game/Gameplay/BP_Asteroid.BP_Asteroid_C" (Math|Transform|MakeTransform (+ (Math|Vector|MakeVector (Math|Random|RandomFloatinRange 1e+02 9e+02) (Math|Random|RandomFloatinRange -5e+02 5e+02) 0.0) (Transformation|GetWorldLocation (Variables|Default|GetDefaultSceneRoot)))) "Undefined" 0 0))
    (Utilities|Array|Add (Variables|Default|GetAsteroids) _returnvalue)))

(fn UpdateLocation
  (params (Location :type Vector))
  (Transformation|AddRelativeLocation (Variables|Default|GetDefaultSceneRoot) Location false false)
  (for _array_element (Variables|Default|GetAsteroids)
    (Transformation|AddRelativeLocation (Variables|/Game/Gameplay/BP_Asteroid.BP_Asteroid_C|GetAsteroid _array_element) Location false false)))