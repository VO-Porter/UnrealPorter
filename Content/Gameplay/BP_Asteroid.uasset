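; BP_Asteroid is an asteroid obstacle that ends the game when the player ship touches it.
; On BeginPlay it gives its Asteroid component a random yaw for visual variety.
; When that component overlaps BP_PlayerShip, it copies TimeElapsed from BP_GameState into LastScore on BP_GameInstance, so the score survives the level change, then opens GameOverLevel.
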(event OnComponentBeginOverlap(Asteroid)
  (params (OverlappedComponent :type Primitive%20Component%20Object%20Reference) (OtherActor :type Actor%20Object%20Reference) (OtherComp :type Primitive%20Component%20Object%20Reference) (OtherBodyIndex :type Integer) (bFromSweep :type Boolean) (SweepResult :type Hit%20Result%20Structure%20%28by%20ref%29))
  (Utilities|Casting|CastToBP_PlayerShip OtherActor)
  (bind _asbp_game_state (Utilities|Casting|CastToBP_GameState (Game|GetGameState)))
  (bind _asbp_game_instance (Utilities|Casting|CastToBP_GameInstance (Game|GetGameInstance)))
  (Variables|/Game/Gameplay/BP_GameInstance.BP_GameInstance_C|SetLastScore _asbp_game_instance (Variables|/Game/Gameplay/BP_GameState.BP_GameState_C|GetTimeElapsed _asbp_game_state))
  (Game|OpenLevel(byName) "GameOverLevel"))

(event EventBeginPlay
  (Transformation|SetRelativeRotation (Variables|Default|GetAsteroid) (Math|Rotator|MakeRotator 0.0 0.0 (Math|Random|RandomFloatinRange 0.0 3.6e+02)) false false))

(event EventTick
  (params (DeltaSeconds :type Float%20%28single-precision%29)))

(fn ConstructionScript)