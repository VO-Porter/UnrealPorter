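; Player ship that slides sideways along world Y and hops on Space, steered with raw K and L key events.
; Tick eases roll and lateral speed toward targets with per-frame Lerps, banking into turns and drifting back to level and rest on release.
; Jumps apply hand-rolled velocity and gravity to the Cube component without sweeps, then a recovery phase eases it back to hover height after it dips below a floor threshold.
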(event EventBeginPlay
  (Input|EnableInput (Game|GetPlayerController 0)))

(event Collision|EventActorBeginOverlap
  (params (OtherActor :type Actor%20Object%20Reference)))

(event EventTick
  (params (DeltaSeconds :type Float%20%28single-precision%29))
  (CallFunction|HandleRotation)
  (CallFunction|HandleMovement)
  (CallFunction|HandleJump))

(event Input|KeyboardEvents|SpaceBar
  (params (Key :type Key%20Structure :default "AnyKey"))
  (:Pressed
    (if (not (or (Variables|Default|GetIsJumping) (Variables|Default|GetIsRecovering)))
      (Variables|Default|SetIsJumping true)
      (Variables|Default|SetJumpVelocity 2e+01))))

(event Input|KeyboardEvents|K
  (params (Key :type Key%20Structure :default "AnyKey"))
  (:Pressed
    (Variables|Default|SetIsMovingLeft true))
  (:Released
    (Variables|Default|SetIsMovingLeft false)))

(event Input|KeyboardEvents|L
  (params (Key :type Key%20Structure :default "AnyKey"))
  (:Pressed
    (Variables|Default|SetIsMovingRight true))
  (:Released
    (Variables|Default|SetIsMovingRight false)))

(fn ConstructionScript)

(fn HandleRotation
  (bind _cube (Variables|Default|GetCube))
  (bind _cube_2 (Variables|Default|GetCube))
  (bind _cube_3 (Variables|Default|GetCube))
  (Utilities|FlowControl|Sequence
    (:then_0
      (if (Variables|Default|GetIsMovingLeft)
        (Transformation|SetRelativeRotation _cube_2 (Math|Rotator|MakeRotator (Math|Float|Lerp (.Roll (Math|Rotator|BreakRotator (Variables|/Script/Engine.SceneComponent|GetRelativeRotation _cube_2))) -3e+01 0.2) 0.0 0.0) false false)))
    (:then_1
      (if (Variables|Default|GetIsMovingRight)
        (Transformation|SetRelativeRotation _cube_3 (Math|Rotator|MakeRotator (Math|Float|Lerp (.Roll (Math|Rotator|BreakRotator (Variables|/Script/Engine.SceneComponent|GetRelativeRotation _cube_3))) 3e+01 0.2) 0.0 0.0) false false)))
    (:then_2
      (if (not (or (Variables|Default|GetIsMovingLeft) (Variables|Default|GetIsMovingRight)))
        (Transformation|SetRelativeRotation _cube (Math|Rotator|MakeRotator (Math|Float|Lerp (.Roll (Math|Rotator|BreakRotator (Variables|/Script/Engine.SceneComponent|GetRelativeRotation _cube))) 0.0 0.05) 0.0 0.0) false false)))))

(fn HandleMovement
  (Utilities|FlowControl|Sequence
    (:then_0
      (if (Variables|Default|GetIsMovingLeft)
        (Variables|Default|SetMovementSpeed (Math|Float|Lerp (Variables|Default|GetMovementSpeed) (- 0.0 (Variables|Default|GetMaxMovementSpeed)) 0.1))))
    (:then_1
      (if (Variables|Default|GetIsMovingRight)
        (Variables|Default|SetMovementSpeed (Math|Float|Lerp (Variables|Default|GetMovementSpeed) (Variables|Default|GetMaxMovementSpeed) 0.1))))
    (:then_2
      (if (not (or (Variables|Default|GetIsMovingLeft) (Variables|Default|GetIsMovingRight)))
        (Variables|Default|SetMovementSpeed (Math|Float|Lerp (Variables|Default|GetMovementSpeed) 0.0 0.03))))
    (:then_3
      (Transformation|AddWorldOffset (Variables|Default|GetCube) (Math|Vector|MakeVector 0.0 (Variables|Default|GetMovementSpeed) 0.0) false false))))

(fn HandleJump
  (bind _cube (Variables|Default|GetCube))
  (bind _returnvalue (Transformation|GetWorldLocation _cube))
  (bind (_x _y _z) (Math|Vector|BreakVector _returnvalue))
  (bind _returnvalue_2 (Math|Float|Lerp _z 1.2e+02 0.25))
  (if (Variables|Default|GetIsJumping)
    (Transformation|AddWorldOffset (Variables|Default|GetCube) (Math|Vector|MakeVector 0.0 0.0 (Variables|Default|GetJumpVelocity)) false false)
    (Variables|Default|SetJumpVelocity (- (Variables|Default|GetJumpVelocity) (Variables|Default|GetGravity)))
    (if (< (.Z (Math|Vector|BreakVector (Transformation|GetWorldLocation (Variables|Default|GetCube)))) 1e+02)
      (Variables|Default|SetIsJumping false)
      (Variables|Default|SetIsRecovering true))
    (elif (Variables|Default|GetIsRecovering)
      (Transformation|SetWorldLocation _cube (Math|Vector|MakeVector _x _y _returnvalue_2) false false)
      (if (Math|Float|NearlyEqual(Float) _returnvalue_2 1.2e+02 0.01)
        (Variables|Default|SetIsRecovering false)))))